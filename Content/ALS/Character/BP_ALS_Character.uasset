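; BP_ALS_Character is a player character with Enhanced Input look, movement, aiming and weapon switching, plus slow-motion debug keys.
; Weapon switching sets EquippedGun and links the matching unarmed, pistol or rifle animation layer class onto the mesh.
; Aim press and release switch the gate through SetCurrentGate, which applies that gate's speed, acceleration and braking values from the GateSettings map and notifies the AnimInstance.
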(event Input|EnhancedActionEvents|EnhancedInputActionIA_SwitchWeapon
  (params (ActionValue :type Float%20%28double-precision%29) (ElapsedSeconds :type Float%20%28double-precision%29) (TriggeredSeconds :type Float%20%28double-precision%29) (InputAction :type Input%20Action%20Object%20Reference :default "/Game/Input/InputActions/IA_SwitchWeapon.IA_SwitchWeapon"))
  ;[1 1 1] Switch weapon
  (:Started
    (bind _output_get (Variables|Default|SetEquippedGun (Utilities|Enum|ByteToEnumE_Guns (- (Math|Conversions|ToByte(Integer) (Class|KismetMathLibrary|ToInt64(Float) ActionValue)) 1))))
    (Development|PrintString (Utilities|String|EnumtoString _output_get))
    (Components|SkeletalMesh|AnimationBlueprintLinking|LinkAnimClassLayers (Variables|Character|GetMesh) (Utilities|Select :Index (Variables|Default|GetEquippedGun) :NewEnumerator0 "/Game/ALS/AnimationBPs/ABP_Unarmed.ABP_Unarmed_C" :NewEnumerator1 "/Game/ALS/AnimationBPs/ABP_Pistol.ABP_Pistol_C" :NewEnumerator2 "/Game/ALS/AnimationBPs/ABP_Rifle.ABP_Rifle_C"))))

(event Input|EnhancedActionEvents|EnhancedInputActionIA_Look
  (params (ActionValue :type Vector%202D%20Structure) (ElapsedSeconds :type Float%20%28double-precision%29) (TriggeredSeconds :type Float%20%28double-precision%29) (InputAction :type Input%20Action%20Object%20Reference :default "/Game/Input/InputActions/IA_Look.IA_Look"))
  (bind (_x _y) (Math|Vector2D|BreakVector2D ActionValue))
  ;[1 1 1] Look and Move
  (Pawn|Input|AddControllerYawInput _x)
  (Pawn|Input|AddControllerPitchInput _y))

(event Input|EnhancedActionEvents|EnhancedInputActionIA_Move
  (params (ActionValue :type Vector%202D%20Structure) (ElapsedSeconds :type Float%20%28double-precision%29) (TriggeredSeconds :type Float%20%28double-precision%29) (InputAction :type Input%20Action%20Object%20Reference :default "/Game/Input/InputActions/IA_Move.IA_Move"))
  (bind (_x _y) (Math|Vector2D|BreakVector2D ActionValue))
  (bind _returnvalue (Pawn|GetControlRotation :!class /Script/Engine.Pawn))
  ;[1 1 1] Look and Move
  (Pawn|Input|AddMovementInput (Math|Vector|GetRightVector (Math|Rotator|MakeRotator (.roll _returnvalue) 0.0 (.yaw _returnvalue))) _x false)
  (Pawn|Input|AddMovementInput (Math|Vector|GetForwardVector (Math|Rotator|MakeRotator 0.0 0.0 (.yaw (Pawn|GetControlRotation :!class /Script/Engine.Pawn)))) _y false))

(event Input|EnhancedActionEvents|EnhancedInputActionIA_Aim
  (params (ActionValue :type Boolean) (ElapsedSeconds :type Float%20%28double-precision%29) (TriggeredSeconds :type Float%20%28double-precision%29) (InputAction :type Input%20Action%20Object%20Reference :default "/Game/Input/InputActions/IA_Aim.IA_Aim"))
  (:Started
    (CallFunction|SetCurrentGate "NewEnumerator0"))
  (:Completed
    (CallFunction|SetCurrentGate "NewEnumerator1")))

(event EventBeginPlay
  ;[1 1 1] Begin play
  (bind _asplayer_controller (Utilities|Casting|CastToPlayerController (Pawn|GetController)))
  (Input|AddMappingContext (PlayerController|LocalPlayerSubsystems|GetEnhancedInputLocalPlayerSubsystem _asplayer_controller) "/Game/Input/IMC_ALS.IMC_ALS" 0 "(bIgnoreAllPressedKeysUntilRelease=True,bForceImmediately=False,bNotifyUserSettings=False)")
  (Components|SkeletalMesh|AnimationBlueprintLinking|LinkAnimClassLayers (Variables|Character|GetMesh) "/Game/ALS/AnimationBPs/ABP_Unarmed.ABP_Unarmed_C")
  (CallFunction|SetCurrentGate "NewEnumerator1"))

(event Input|KeyboardEvents|DebugKeySubtract
  (params (Key :type Key%20Structure :default "None") (ActionValue :type Input%20Action%20Value%20Structure))
  ;[1 0.6354 0.8595] Debug slomo
  (:Pressed
    (Utilities|Time|SetGlobalTimeDilation 0.1)))

(event Input|KeyboardEvents|DebugKeyAdd
  (params (Key :type Key%20Structure :default "None") (ActionValue :type Input%20Action%20Value%20Structure))
  ;[1 0.6354 0.8595] Debug slomo
  (:Pressed
    (Utilities|Time|SetGlobalTimeDilation 1.0)))

(fn ConstructionScript)

(fn SetCurrentGate
  (params (CurrentGate :type E_Gate%20Enum :default "NewEnumerator0"))
  (bind _output_get (Variables|Default|SetCurrentGate CurrentGate))
  (Utilities|FlowControl|Sequence
    (:then_0
      (Variables|/Script/Engine.CharacterMovementComponent|SetMaxWalkSpeed (Variables|Character|GetCharacterMovement) (.MaxWalkSpeed (Utilities|Struct|BreakS_GateSetting (.Value (Utilities|Map|Find (Variables|Default|GetGateSettings) _output_get))))))
    (:then_1
      (Variables|/Script/Engine.CharacterMovementComponent|SetMaxAcceleration (Variables|Character|GetCharacterMovement) (.MaxAcceleration (Utilities|Struct|BreakS_GateSetting (.Value (Utilities|Map|Find (Variables|Default|GetGateSettings) _output_get))))))
    (:then_2
      (Variables|/Script/Engine.CharacterMovementComponent|SetBrakingDecelerationWalking (Variables|Character|GetCharacterMovement) (.BrakingDeceleration (Utilities|Struct|BreakS_GateSetting (.Value (Utilities|Map|Find (Variables|Default|GetGateSettings) _output_get))))))
    (:then_3
      (Variables|/Script/Engine.CharacterMovementComponent|SetBrakingFrictionFactor (Variables|Character|GetCharacterMovement) (.BrakingFrictionFactor (Utilities|Struct|BreakS_GateSetting (.Value (Utilities|Map|Find (Variables|Default|GetGateSettings) _output_get))))))
    (:then_4
      (Variables|/Script/Engine.CharacterMovementComponent|SetBrakingFriction (Variables|Character|GetCharacterMovement) (.BrakingFriction (Utilities|Struct|BreakS_GateSetting (.Value (Utilities|Map|Find (Variables|Default|GetGateSettings) _output_get))))))
    (:then_5
      (Variables|/Script/Engine.CharacterMovementComponent|SetbUseSeparateBrakingFriction (Variables|Character|GetCharacterMovement) (.UseSeparateBrakingFriction (Utilities|Struct|BreakS_GateSetting (.Value (Utilities|Map|Find (Variables|Default|GetGateSettings) _output_get))))))
    (:then_6
      (Class|BPIAnimInterface|UpdateCurrentGate(Message) (Components|SkeletalMesh|GetAnimInstance (Variables|Character|GetMesh)) (Variables|Default|GetCurrentGate)))))